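; BP_Item is a pickup item actor that the FPS player can equip as a radio or flashlight.
; Trigger overlaps register or clear it as the player's CurrentItem and toggle the pickup hint, which PickUp hides a tick later.
; EquipToPlayer copies ItemModel onto the matching player socket mesh, then hides the actor and disables its collision.
; The construction script applies ItemModel to MeshItem, so item variants need no duplicate Blueprint.
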(event OnComponentBeginOverlap(Trigger)
  (params (OverlappedComponent :type Primitive%20Component%20Object%20Reference) (OtherActor :type Actor%20Object%20Reference) (OtherComp :type Primitive%20Component%20Object%20Reference) (OtherBodyIndex :type Integer) (bFromSweep :type Boolean) (SweepResult :type Hit%20Result%20Structure%20%28by%20ref%29))
  (bind _asbp_fps_player (Utilities|Casting|CastToBP_FPS_Player OtherActor))
  (Variables|/Game/LD59/Blueprint/Player/BP_FPS_Player.BP_FPS_Player_C|SetCurrentItem _asbp_fps_player self)
  (Default|ShowPickupHint _asbp_fps_player true))

(event OnComponentEndOverlap(Trigger)
  (params (OverlappedComponent :type Primitive%20Component%20Object%20Reference) (OtherActor :type Actor%20Object%20Reference) (OtherComp :type Primitive%20Component%20Object%20Reference) (OtherBodyIndex :type Integer))
  (bind _asbp_fps_player (Utilities|Casting|CastToBP_FPS_Player OtherActor))
  (if (== (Variables|/Game/LD59/Blueprint/Player/BP_FPS_Player.BP_FPS_Player_C|GetCurrentItem _asbp_fps_player) 0)
    (Variables|/Game/LD59/Blueprint/Player/BP_FPS_Player.BP_FPS_Player_C|SetCurrentItem _asbp_fps_player 0)
    (Default|ShowPickupHint _asbp_fps_player false)))

(event EventPickUp
  ;[0.15 0.15 0.15 0.5] Delete widget "E to pickup" on Pickup
  (Utilities|FlowControl|DelayUntilNextTick)
  (bind _asbp_fps_player (Utilities|Casting|CastToBP_FPS_Player (Pawn|GetControlledPawn (Game|GetPlayerController 0))))
  (Default|ShowPickupHint _asbp_fps_player false))

(event Collision|EventActorEndOverlap
  (params (OtherActor :type Actor%20Object%20Reference))
  (bind _asbp_fps_player (Utilities|Casting|CastToBP_FPS_Player OtherActor))
  (if (== (Variables|/Game/LD59/Blueprint/Player/BP_FPS_Player.BP_FPS_Player_C|GetCurrentItem _asbp_fps_player) self)
    (Variables|/Game/LD59/Blueprint/Player/BP_FPS_Player.BP_FPS_Player_C|SetCurrentItem _asbp_fps_player 0)))

(fn ConstructionScript
  (bind _mesh_item (Variables|Default|GetMesh_Item))
  ;[0.15 0.15 0.15 0.5] Logic to duplicate mesh without duplicating BP
  (if (Utilities|IsValid _mesh_item)
    (Components|StaticMesh|SetStaticMesh _mesh_item (Variables|Default|GetItemModel))))

(fn GetItem
  (params (Player :type BP%20FPS%20Player%20Object%20Reference))
  (for _array_element (Collision|GetOverlappingActors Player "BP_Item_C" :!class /Script/Engine.Actor)
    (if (Utilities|DoesObjectImplementInterface _array_element "/Game/LD59/Blueprint/Items/BPI_Items.BPI_Items_C")
      (return _array_element))))

(fn EquiptoPlayer
  (params (Player :type BP%20FPS%20Player%20Object%20Reference) (EquipSlot :type E_EquipSlot%20Enum :default "NewEnumerator0"))
  (bind _itemmodel (Variables|Default|GetItemModel))
  ;[0.2051 0.01521 0.3005] EquipToPlayer Pick up logic
  (if (Utilities|IsValid Player)
    (switch Utilities|FlowControl|Switch|SwitchonE_EquipSlot EquipSlot
      (:NewEnumerator0
        (Components|StaticMesh|SetStaticMesh (Variables|/Game/LD59/Blueprint/Player/BP_FPS_Player.BP_FPS_Player_C|GetSocket_Radio Player) _itemmodel))
      (:NewEnumerator1
        (Components|StaticMesh|SetStaticMesh (Variables|/Game/LD59/Blueprint/Player/BP_FPS_Player.BP_FPS_Player_C|GetSocket_FlashLight Player) _itemmodel)))
    (Rendering|SetActorHiddenInGame true)
    (Collision|SetActorEnableCollision false)))